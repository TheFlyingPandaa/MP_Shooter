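; Superspeed power-up actor that temporarily doubles the walk speed of the actor that activates it.
; On activation it stores that actor and sets its CharacterMovementComponent MaxWalkSpeed to twice the current GetMaxSpeed.
; On expiry it sets MaxWalkSpeed to half the then-current GetMaxSpeed if the actor is still valid, rather than restoring a cached value, then calls the parent expiry logic.
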(event `self.OnActivated`
  (params (OtherActor :type "Actor Object Reference"))
  (bind _returnvalue (`self.GetComponentByClass` (`self.Powered Actor`) "/Script/Engine.CharacterMovementComponent"))
  (set `self.Powered Actor` OtherActor)
  (set `CharacterMovementComponent.MaxWalkSpeed` (* (`MovementComponent.GetMaxSpeed` _returnvalue) 2.0) _returnvalue))

(event `self.OnExpired`
  (bind _powered_actor (`self.Powered Actor`))
  (bind _returnvalue (`self.GetComponentByClass` _powered_actor "/Script/Engine.CharacterMovementComponent"))
  (`/Engine/EditorBlueprintResources/StandardMacros.IsValid` _powered_actor
    (:`Is Valid`
      (set `CharacterMovementComponent.MaxWalkSpeed` (* (`MovementComponent.GetMaxSpeed` _returnvalue) 0.5) _returnvalue))
    (:`Is Not Valid`
      _))
  (`parent.OnExpired`))

(fn `UserConstructionScript`)