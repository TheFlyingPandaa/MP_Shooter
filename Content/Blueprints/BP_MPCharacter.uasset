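; Multiplayer player character Blueprint that sets up the local HUD and tracks the player's gold.
; On BeginPlay, only the locally controlled instance creates crosshair, health indicator and temporary HUD widgets.
; GiveGold adds to and prints the Gold total.
; Debug keys print lane HP through MPGameMode (Q) and raise the current weapon's damage when Store1 is set (I).
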(event `self.ReceiveBeginPlay`
  (if (`self.IsLocallyControlled`)
    (`|ExecutionSequence`
      (:`then_0`
        (bind _returnvalue (`|CreateWidget` "/Game/UI/WBP_Crosshair.WBP_Crosshair_C"))
        (`UserWidget.AddToViewport` _returnvalue 0))
      (:`then_1`
        (bind _returnvalue_2 (`|CreateWidget` "/Game/UI/WBP_HealthIndicator.WBP_HealthIndicator_C"))
        (`UserWidget.AddToViewport` _returnvalue_2 0))
      (:`then_2`
        (bind _returnvalue_3 (`|CreateWidget` "/Game/Blueprints/TempHud/BP_TempHud.BP_TempHud_C"))
        (`UserWidget.AddToViewport` _returnvalue_3 0)))))

(event `Key|Q`
  (params (Key :type "Key Structure"))
  ;[1 1 1] Debug: Print all lane HP
  (:`Pressed`
    (bind _asmpgame_mode (cast `/Game/Blueprints/MPGameMode` (`GameplayStatics.GetGameMode`)))
    (`/Game/Blueprints/MPGameMode.PrintHP` _asmpgame_mode)))

(event `Key|I`
  (params (Key :type "Key Structure"))
  (bind _currentweapon (`self.CurrentWeapon`))
  (bind _weapondamage (`MPWeapon.WeaponDamage` _currentweapon))
  ;[1 1 1] Debug: Increase damage
  (:`Pressed`
    (if (`self.Store1`)
      (set `MPWeapon.WeaponDamage` (+ _weapondamage 10.0) _currentweapon)
      (`KismetSystemLibrary.PrintString` (`KismetStringLibrary.Conv_DoubleToString` _weapondamage)))))

(event `GiveGold`
  (params (GoldInput :type Integer))
  (bind _output_get (set `self.Gold` (+ GoldInput (`self.Gold`))))
  (`KismetSystemLibrary.PrintString` (`KismetStringLibrary.Conv_IntToString` _output_get)))

(fn `UserConstructionScript`)