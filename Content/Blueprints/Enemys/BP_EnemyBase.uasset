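; Base enemy Blueprint that handles taking damage, dying and rewarding gold for the kill.
; AnyDamage subtracts damage from Health and, at zero or below, spawns a death particle at the actor's location and destroys it.
; It then casts the damage causer to BP_MPWeaponRifle to call GiveGold with a fixed amount, so other causers only trigger a debug print.
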(event `self.ReceiveAnyDamage`
  (params (Damage :type "Float (single-precision)") (DamageType :type "DamageType Object Reference") (InstigatedBy :type "Controller Object Reference") (DamageCauser :type "Actor Object Reference"))
  ;[1 1 1] Takeing Damage logic
  (set `self.Health` (- (`self.Health`) Damage))
  (if (<= (`self.Health`) 0.0)
    (`GameplayStatics.SpawnEmitterAtLocation` "/Game/StarterContent/Particles/P_deathParticle.P_deathParticle" (`self.K2_GetActorLocation`))
    (`self.K2_DestroyActor`)
    ;[0.1188 1 0.1619] Give gold to player
    (bind _asbp_mpweapon_rifle (cast `/Game/Blueprints/BP_MPWeaponRifle` DamageCauser)
      (:`then`
        (`/Game/Blueprints/BP_MPWeaponRifle.GiveGold` _asbp_mpweapon_rifle 10))
      (:`CastFailed`
        (`KismetSystemLibrary.PrintString` "GOLD CAST FAILD. SIMPLE ENEMY" true true (struct :`R` 1.0 :`G` 0.009009 :`A` 1.0))))))

(fn `UserConstructionScript`)