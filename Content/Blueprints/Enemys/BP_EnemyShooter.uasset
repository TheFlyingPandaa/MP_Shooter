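; BP_EnemyShooter is an enemy character that fires projectiles at a focused player.
; While PlayerFocusBool is set, Tick casts PlayerFocus to BP_MPCharacter, snaps the enemy's rotation toward it and halts movement.
; It spawns a FirstPersonProjectile at ProjectileSpawn and launches it with an impulse along the mesh's forward vector, using a flag and Delay as cooldown.
; The focus variables are not set in this graph.
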(event `self.ReceiveBeginPlay`
  (`parent.ReceiveBeginPlay`))

(event `self.ReceiveTick`
  (params (DeltaSeconds :type "Float (single-precision)"))
  (`parent.ReceiveTick` DeltaSeconds)
  (if (`self.PlayerFocusBool`)
    (bind _asbp_mpcharacter (cast `/Game/Blueprints/Characters/BP_MPCharacter` (`self.PlayerFocus`))
      (:`then`
        (`|ExecutionSequence`
          (:`then_0`
            (`self.K2_SetActorRotation` (`KismetMathLibrary.FindLookAtRotation` (`self.K2_GetActorLocation`) (`self.K2_GetActorLocation` _asbp_mpcharacter)))
            (`MovementComponent.StopMovementImmediately` (`self.CharacterMovement`)))
          (:`then_1`
            (if (`self.canSpawnProj`)
              (bind _returnvalue (`|SpawnActorFromClass` "/Game/FirstPersonBP/Blueprints/FirstPersonProjectile.FirstPersonProjectile_C" (`SceneComponent.K2_GetComponentToWorld` (`self.ProjectileSpawn`)) "Undefined" "OverrideRootScale" null null))
              (`PrimitiveComponent.AddImpulse` (`/Game/FirstPersonBP/Blueprints/FirstPersonProjectile.CollisionComponent` _returnvalue) (* (`SceneComponent.GetForwardVector` (`self.Mesh`)) (`self.shootSpeed`)) "None" true)
              (set `self.canSpawnProj` false)
              (`KismetSystemLibrary.Delay` 1.5)
              (set `self.canSpawnProj` true)))))
      (:`CastFailed`
        (`KismetSystemLibrary.PrintString` "FUCK")))))

(fn `UserConstructionScript`
  (`parent.UserConstructionScript`))