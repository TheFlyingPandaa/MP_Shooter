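; BP_SimpleEnemy is a basic enemy that chases players and can be killed by damage.
; When PawnSensing sees a BP_MPCharacter, it moves toward that character with AIMoveTo.
; Any damage reduces its Health, printing the remaining value until zero, when it spawns an explosion emitter and destroys itself.
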(event `self.PawnSensing.OnSeePawn`
  (params (Pawn :type "Pawn Object Reference"))
  (bind _asbp_mpcharacter (cast `/Game/Blueprints/BP_MPCharacter` Pawn))
  (`|AIMoveTo` self (0.0 0.0 0.0) _asbp_mpcharacter))

(event `self.ReceiveAnyDamage`
  (params (Damage :type "Float (single-precision)") (DamageType :type "DamageType Object Reference") (InstigatedBy :type "Controller Object Reference") (DamageCauser :type "Actor Object Reference"))
  (bind _health (`self.Health`))
  (set `self.Health` (- (`self.Health`) Damage))
  (if (<= _health 0.0)
    (`GameplayStatics.SpawnEmitterAtLocation` "/Game/StarterContent/Particles/P_Explosion.P_Explosion" (`self.K2_GetActorLocation`))
    (`self.K2_DestroyActor`)
    (else
      (`KismetSystemLibrary.PrintString` (`KismetStringLibrary.Conv_DoubleToString` _health)))))

(fn `UserConstructionScript`)