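; Multiplayer player character Blueprint for Murdock that handles local HUD, inventory, store and gold.
; On BeginPlay the locally controlled pawn creates crosshair, health indicator and temporary HUD widgets.
; The I key toggles the inventory, adding the store widget when the store flag is set, and GiveGold increases the gold total.
; Debug keys print lane HP through GameplayGameMode or, with the store flag, raise weapon damage and add an inventory item.
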(event `self.ReceiveBeginPlay`
  (if (`self.IsLocallyControlled`)
    (`|ExecutionSequence`
      (:`then_0`
        (bind _returnvalue (`|CreateWidget` "/Game/UI/Gameplay/WBP_Crosshair.WBP_Crosshair_C"))
        (`UserWidget.AddToViewport` _returnvalue 0))
      (:`then_1`
        (bind _returnvalue_2 (`|CreateWidget` "/Game/UI/Gameplay/WBP_HealthIndicator.WBP_HealthIndicator_C"))
        (`UserWidget.AddToViewport` _returnvalue_2 0))
      (:`then_2`
        (bind _returnvalue_3 (`|CreateWidget` "/Game/Blueprints/TempHud/BP_TempHud.BP_TempHud_C"))
        (`UserWidget.AddToViewport` _returnvalue_3 0)))))

(event `Key|Q`
  (params (Key :type "Key Structure"))
  ;[1 1 1] Debug: Print all lane HP
  (:`Pressed`
    (bind _asgameplay_game_mode (cast `/Game/Blueprints/Gameplay/GameplayGameMode` (`GameplayStatics.GetGameMode`)))
    (`/Game/Blueprints/Gameplay/GameplayGameMode.PrintHP` _asgameplay_game_mode)))

(event `Key|I`
  (params (Key :type "Key Structure"))
  (bind _ui_store_1 (`self.UI_Store_1`))
  ;[1 1 1] Inventory Opening
  (:`Pressed`
    (if (`self.InventoryOpen_0`)
      (`Widget.RemoveFromParent` (`self.UI_inventory_0`))
      (set `self.InventoryOpen_0` false)
      (if (`KismetSystemLibrary.IsValid` _ui_store_1)
        (`Widget.RemoveFromParent` _ui_store_1))
      (else
        (bind _returnvalue (`|CreateWidget` "/Game/Blueprints/Inventory/UI_Inventory.UI_Inventory_C"))
        (set `self.UI_inventory_0` _returnvalue)
        (`UserWidget.AddToViewport` _returnvalue 0)
        (set `self.InventoryOpen_0` true)
        (if (`self.Store1_0`)
          (bind _returnvalue_2 (`|CreateWidget` "/Game/Blueprints/Store/UI_Store.UI_Store_C"))
          (set `self.UI_Store_1` _returnvalue_2)
          (`UserWidget.AddToViewport` _returnvalue_2 0))))))

(event `Key|O`
  (params (Key :type "Key Structure"))
  (bind _currentweapon (`self.CurrentWeapon`))
  (bind _weapondamage (`MPWeapon.WeaponDamage` _currentweapon))
  ;[1 1 1] Debug: Increase damage
  (:`Pressed`
    (if (`self.Store1_0`)
      (set `MPWeapon.WeaponDamage` (+ _weapondamage 10.0) _currentweapon)
      (`KismetSystemLibrary.PrintString` (`KismetStringLibrary.Conv_DoubleToString` _weapondamage))
      (`KismetArrayLibrary.Array_Add` (`self.Inventory_0`) (make `/Game/Blueprints/Inventory/Inventory_Struct` 1 "Weapon" "/Game/WeaponEffects/BasicTracer/Beam.Beam"))
      (if (`self.InventoryOpen_0`)
        (`Widget.RemoveFromParent` (`self.UI_inventory_0`))
        (bind _returnvalue (`|CreateWidget` "/Game/Blueprints/Inventory/UI_Inventory.UI_Inventory_C"))
        (set `self.UI_inventory_0` _returnvalue)
        (`UserWidget.AddToViewport` _returnvalue 0)))))

(event `GiveGold`
  (params (GoldInput :type Integer))
  (bind _output_get (set `self.Gold_0` (+ GoldInput (`self.Gold_0`))))
  (`KismetSystemLibrary.PrintString` (`KismetStringLibrary.Conv_IntToString` _output_get)))

(fn `UserConstructionScript`)