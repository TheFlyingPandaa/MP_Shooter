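; BP_SimpleEnemy is a basic AI enemy that heads for KillActor, a death zone, unless it sees a player to chase.
; PawnSensing sets a focus flag and target, Tick reissues AIMoveTo accordingly, and a retriggerable delay in Tick clears the flag.
; Damage lowers Health; at zero it spawns a death particle, destroys itself and grants gold through the damage causer if that is a BP_MPWeaponRifle.
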(event `self.ReceiveTick`
  (params (DeltaSeconds :type "Float (single-precision)"))
  (if (`self.PlayerFocusBool`)
    (`|ExecutionSequence`
      (:`then_0`
        ;[1 1 1] If we se a player. Move to the player
        (bind _asbp_mpcharacter (cast `/Game/Blueprints/Characters/BP_MPCharacter` (`self.PlayerFocus`)))
        (`|AIMoveTo` self (0.0 0.0 0.0) _asbp_mpcharacter))
      (:`then_1`
        (`KismetSystemLibrary.RetriggerableDelay` 0.5)
        (set `self.PlayerFocusBool` false)))
    (else
      ;[1 1 1] If no player, then go for death zone
      (`|AIMoveTo` self (0.0 0.0 0.0) (`self.KillActor`)))))

(event `self.PawnSensing.OnSeePawn`
  (params (Pawn :type "Pawn Object Reference"))
  ;[1 1 1] Player sensing.
  (set `self.PlayerFocus` Pawn)
  (set `self.PlayerFocusBool` true))

(event `self.ReceiveAnyDamage`
  (params (Damage :type "Float (single-precision)") (DamageType :type "DamageType Object Reference") (InstigatedBy :type "Controller Object Reference") (DamageCauser :type "Actor Object Reference"))
  (bind _health (`self.Health`))
  ;[1 1 1] Takeing Damage logic
  (set `self.Health` (- (`self.Health`) Damage))
  (if (<= _health 0.0)
    (`GameplayStatics.SpawnEmitterAtLocation` "/Game/StarterContent/Particles/P_deathParticle.P_deathParticle" (`self.K2_GetActorLocation`))
    (`self.K2_DestroyActor`)
    ;[0.1188 1 0.1619] Give gold to player
    (bind _asbp_mpweapon_rifle (cast `/Game/Blueprints/BP_MPWeaponRifle` DamageCauser)
      (:`then`
        (`/Game/Blueprints/BP_MPWeaponRifle.GiveGold` _asbp_mpweapon_rifle 10))
      (:`CastFailed`
        (`KismetSystemLibrary.PrintString` "GOLD CAST FAILD. SIMPLE ENEMY" true true (struct :`R` 1.0 :`G` 0.009009 :`A` 1.0))))
    (else
      (`KismetSystemLibrary.PrintString` (`KismetStringLibrary.Conv_DoubleToString` _health)))))

(fn `UserConstructionScript`)