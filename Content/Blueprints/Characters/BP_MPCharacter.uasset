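; Multiplayer player character Blueprint that handles crosshair and HUD creation, inventory UI input and debug keys.
; L toggles a spawn inventory, creating a new inventory actor with a spawner item and a new widget on each open.
; InventoryInput maps numpad keys to slot indices for the open inventory widget.
; Tick drives an income timer that only resets; gold, main inventory setup and damage boost logic are stubbed or disconnected.
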(event `InputAction|InventoryInput`
  (params (Key :type "Key Structure"))
  ;[1 1 1] Widget Input
  (:`Pressed`
    (bind _keynumber (`self.getInventoryKeyInput` Key))
    (if (and (`self.SpawnOpen`) (`KismetSystemLibrary.IsValid` (`self.UI_SpawnInventory`)))
      (`/Game/rInventory/Widgets/UserInterfaceWidget.KeyBoardInput` (`self.UI_SpawnInventory`) _keynumber)
      (elif (and (`self.InventoryOpen`) (`KismetSystemLibrary.IsValid` (`self.UI_Inventory`)))
        (`/Game/rInventory/Widgets/UserInterfaceWidget.KeyBoardInput` (`self.UI_Inventory`) _keynumber)))))

(event `self.ReceiveTick`
  (params (DeltaSeconds :type "Float (single-precision)"))
  (if (>= (`self.Timer`) (`self.IncomeTimer`))
    (`self.GiveIncome`)
    (else
      (set `self.Timer` (+ (`self.Timer`) DeltaSeconds)))))

(event `Key|L`
  (params (Key :type "Key Structure"))
  (bind _returnvalue (`GameplayStatics.GetPlayerController` 0))
  (bind _returnvalue_2 (`GameplayStatics.GetPlayerController` 0))
  (:`Pressed`
    (if (`self.SpawnOpen`)
      (set `self.SpawnOpen` false)
      (`Widget.SetRenderOpacity` (`self.UI_SpawnInventory`) 0.5)
      (set `PlayerController.bShowMouseCursor` false _returnvalue_2)
      (`WidgetBlueprintLibrary.SetInputMode_GameOnly` _returnvalue_2)
      (else
        (set `self.SpawnOpen` true)
        (bind _returnvalue_3 (`|SpawnActorFromClass` "/Game/rInventory/Core/rInventoryActor.rInventoryActor_C" (`KismetMathLibrary.MakeTransform` (0.0 0.0 0.0)) "AdjustIfPossibleButDontSpawnIfColliding" "OverrideRootScale" null 5 null))
        (`KismetSystemLibrary.PrintString` "Hello")
        (`/Game/rInventory/Core/rInventoryActor.AddToInventory` _returnvalue_3 "/Game/rInventory/Items/rItem_Spawner.rItem_Spawner_C" 1 false)
        (bind _returnvalue_4 (`|CreateWidget` "/Game/rInventory/Widgets/UserInterfaceWidget.UserInterfaceWidget_C" null _returnvalue_3 (500.0 900.0)))
        (bind _output_get (set `self.UI_SpawnInventory` _returnvalue_4))
        (`UserWidget.AddToViewport` _output_get 0)
        (set `PlayerController.bShowMouseCursor` true _returnvalue)
        (`WidgetBlueprintLibrary.SetInputMode_GameAndUIEx` _returnvalue _returnvalue_4 "DoNotLock" false)))))

(event `Key|T`
  (params (Key :type "Key Structure"))
  (:`Pressed`
    (`KismetSystemLibrary.PrintString` (`KismetStringLibrary.Conv_DoubleToString` (`MPWeapon.WeaponDamage` (`self.CurrentWeapon`))))))

(event `self.ReceiveBeginPlay`
  (`|ExecutionSequence`
    (:`then_0`
      (bind _returnvalue (`|CreateWidget` "/Game/UI/Gameplay/WBP_Crosshair.WBP_Crosshair_C"))
      (`UserWidget.AddToViewport` _returnvalue 0))
    (:`then_2`
      (bind _returnvalue_2 (`|CreateWidget` "/Game/Blueprints/TempHud/BP_TempHud.BP_TempHud_C"))
      (`UserWidget.AddToViewport` _returnvalue_2 0))))

(event `Key|I`
  (params (Key :type "Key Structure")))

(event `Key|O`
  (params (Key :type "Key Structure"))
  ;[1 1 1] Debug: Increase damage
  (:`Pressed`
    (if (and (`self.Store1`) (>= 0 100))
      _)))

(event `GiveGold`
  (params (GoldInput :type Integer)))

(fn `getInventoryKeyInput`
  (params (InputKey :type "Key Structure"))
  (returns (KeyNumber :type Integer))
  (locals (`Key output` :type Integer))
  (if (== InputKey "NumPadOne")
    (set `local.Key output` 0)
    (elif (== InputKey "NumPadTwo")
      (set `local.Key output` 1)
      (elif (== InputKey "NumPadThree")
        (set `local.Key output` 2)
        (elif (== InputKey "NumPadFour")
          (set `local.Key output` 3)
          (elif (== InputKey "NumPadFive")
            (set `local.Key output` 4)
            (elif (== InputKey "NumPadSix")
              (set `local.Key output` 5)
              (elif (== InputKey "NumPadSeven")
                (set `local.Key output` 6)
                (elif (== InputKey "NumPadEight")
                  (set `local.Key output` 7)
                  (elif (== InputKey "NumPadNine")
                    (set `local.Key output` 8)
                    (else
                      (set `local.Key output` -1)))))))))))
  (return (`local.Key output`)))

(fn `GiveIncome`
  (set `self.Timer` 0.0))

(fn `OnRep_Inventory`)

(fn `UpdateInventoryWidget`
  (params (SpawnPoint :type "Vector2D Structure" :default (100.0 100.0)))
  (`Widget.RemoveFromParent` (`self.UI_Inventory`))
  (bind _returnvalue (`|CreateWidget` "/Game/rInventory/Widgets/UserInterfaceWidget.UserInterfaceWidget_C" null (`self.Inventory`) SpawnPoint))
  (bind _output_get (set `self.UI_Inventory` _returnvalue))
  (`UserWidget.AddToViewport` _output_get 0))

(fn `UserConstructionScript`)