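; Multiplayer game mode child Blueprint that tracks a health value for each lane in an array.
; StartGame runs once behind a GameStarted flag, calling SetBasicInfo to count players and give one lane per player the same starting health.
; DamageLane takes one point off the given lane, and PrintHP prints every lane's index and health for debugging.
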(event `DamageLane`
  (params (Lane :type Integer))
  (`KismetArrayLibrary.Array_Set` (`self.LaneHealth`) Lane (- (`|GetArrayItem` (`self.LaneHealth`) Lane) 1)))

(event `StartGame`
  ;[0.3906 0.3906 0.3906] Game start block
  (if (`self.GameStarted?`)
    (`KismetSystemLibrary.PrintString` "Game already Started")
    (else
      (set `self.GameStarted?` true)
      (`self.setBasicInfo`))))

(event `PrintHP`
  ;[1 1 1] Print HP for every lane
  (for (_array_element _array_index) (`self.LaneHealth`)
    (`KismetSystemLibrary.PrintString` (`KismetStringLibrary.Conv_IntToString` _array_index))
    (`KismetSystemLibrary.PrintString` (`KismetStringLibrary.Conv_IntToString` _array_element))))

(event `self.ReceiveBeginPlay`
  (`parent.ReceiveBeginPlay`))

(event `self.ReceiveTick`
  (params (DeltaSeconds :type "Float (single-precision)"))
  (`parent.ReceiveTick` DeltaSeconds))

(fn `setBasicInfo`
  (bind _returnvalue (`self.GetNumPlayers`))
  (bind _output_get (set `self.AmountOfPlayers` _returnvalue))
  (for _index (range _output_get)
    (`KismetArrayLibrary.Array_Set` (`self.LaneHealth`) _index 50 true)))

(fn `UserConstructionScript`
  (`parent.UserConstructionScript`))