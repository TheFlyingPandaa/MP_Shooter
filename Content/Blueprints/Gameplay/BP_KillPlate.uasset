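; BP_KillPlate is a team-owned kill zone that damages its lane when breached.
; On sphere overlap, the server destroys player-controlled MPCharacters from other teams and calls DamageLane with the plate's TeamID on GameplayGameMode.
; Any overlapping actor that is not an MPCharacter is also destroyed and damages the lane, with no team check.
; The construction script labels the plate with its team ID.
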(event `self.Sphere.OnComponentBeginOverlap`
  (params (OverlappedComponent :type "PrimitiveComponent Object Reference") (OtherActor :type "Actor Object Reference") (OtherComp :type "PrimitiveComponent Object Reference") (OtherBodyIndex :type Integer) (bFromSweep :type Boolean) (SweepResult :type "HitResult Structure (by ref)"))
  (`/Engine/EditorBlueprintResources/ActorMacros.Switch Has Authority`
    (:`Authority`
      (bind _asmpcharacter (cast `MPCharacter` OtherActor)
        (:`then`
          ;[1 1 1] Test if actor is enemy pawn
          (bind _asgameplay_player_controller (cast `/Game/Blueprints/Gameplay/GameplayPlayerController` (`Pawn.GetController` _asmpcharacter))
            (:`then`
              (if (!= (`.MyPlayerTeamID_25_E16B849944202A997D44F69CDF386509` (break `/Game/Blueprints/AllLevels/PlayerInfo` (`/Game/Blueprints/Gameplay/GameplayPlayerController.PlayerSettings` _asgameplay_player_controller))) (`self.TeamID`))
                (`self.K2_DestroyActor` _asmpcharacter)
                (bind _asgameplay_game_mode (cast `/Game/Blueprints/Gameplay/GameplayGameMode` (`GameplayStatics.GetGameMode`) :!label _label))
                (`/Game/Blueprints/Gameplay/GameplayGameMode.DamageLane` _asgameplay_game_mode (`self.TeamID`))))
            (:`CastFailed`
              (`KismetSystemLibrary.PrintString` "Kill plate cast error"))))
        (:`CastFailed`
          (`self.K2_DestroyActor` OtherActor)
          (goto _label))))))

(fn `UserConstructionScript`
  (`TextRenderComponent.K2_SetText` (`self.TextRender1`) (`KismetTextLibrary.Conv_StringToText` (`KismetStringLibrary.Concat_StrStr` "Team: " (`KismetStringLibrary.Conv_IntToString` (`self.TeamID`))))))