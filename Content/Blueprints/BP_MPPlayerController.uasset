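; Multiplayer player controller that turns player input into respawn, enemy spawn and game start requests to MPGameMode.
; Jump requests a respawn when no pawn is controlled, P spawns the configured enemy type, and H starts the game.
; Each input calls a request event that proceeds only with authority, then casts the game mode and calls the matching function.
; Jump also prints debug strings.
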(event `Request GMRespawn`
  (bind _returnvalue (`GameplayStatics.GetGameMode`))
  ;[1 1 1] Request Respawn
  (`/Engine/EditorBlueprintResources/ActorMacros.Switch Has Authority`
    (:`Authority`
      (`/Engine/EditorBlueprintResources/StandardMacros.IsValid` _returnvalue
        (:`Is Valid`
          (bind _asmpgame_mode (cast `/Game/Blueprints/MPGameMode` _returnvalue))
          (`/Engine/EditorBlueprintResources/StandardMacros.IsValid` _asmpgame_mode
            (:`Is Valid`
              (`/Game/Blueprints/MPGameMode.Respawn` _asmpgame_mode self))))))))

(event `InputAction|Jump` :consume false
  (params (Key :type "Key Structure"))
  ;[1 1 1] Respawn
  (:`Pressed`
    (`KismetSystemLibrary.PrintString` "Hello")
    (`/Engine/EditorBlueprintResources/StandardMacros.IsValid` (`self.K2_GetPawn` self)
      (:`Is Valid`
        (`KismetSystemLibrary.PrintString` "PC class still has pawn controlled"))
      (:`Is Not Valid`
        (`self.Request GMRespawn`)))))

(event `Request Enemy Spawn`
  (params (`Enemy To Spawn` :type "Actor Class Reference"))
  (bind _returnvalue (`GameplayStatics.GetGameMode`))
  ;[1 1 1] Request Enemy Spawn
  (`/Engine/EditorBlueprintResources/ActorMacros.Switch Has Authority`
    (:`Authority`
      (`/Engine/EditorBlueprintResources/StandardMacros.IsValid` _returnvalue
        (:`Is Valid`
          (bind _asmpgame_mode (cast `/Game/Blueprints/MPGameMode` _returnvalue))
          (`/Game/Blueprints/MPGameMode.Spawn Enemy` _asmpgame_mode `Enemy To Spawn`))))))

(event `Key|P`
  (params (Key :type "Key Structure"))
  ;[1 1 1] Spawn Enemy
  (:`Pressed`
    (`self.Request Enemy Spawn` (`self.Enemy To Spawn`))))

(event `Key|H`
  (params (Key :type "Key Structure"))
  ;[1 1 1] Start Game
  (:`Pressed`
    (`self.Request Game Start`)))

(event `Request Game Start`
  (bind _returnvalue (`GameplayStatics.GetGameMode`))
  ;[1 1 1] Request Game Start
  (`/Engine/EditorBlueprintResources/ActorMacros.Switch Has Authority`
    (:`Authority`
      (`/Engine/EditorBlueprintResources/StandardMacros.IsValid` _returnvalue
        (:`Is Valid`
          (bind _asmpgame_mode (cast `/Game/Blueprints/MPGameMode` _returnvalue))
          (`/Game/Blueprints/MPGameMode.StartGame` _asmpgame_mode))))))

(fn `UserConstructionScript`)