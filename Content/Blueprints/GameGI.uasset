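; GameGI, apparently the game instance, handles multiplayer session hosting and joining along with the menus for both.
; It lazily creates and caches the search and host widgets, then adds them to the viewport.
; LaunchLobby stores the server name, creates a non-LAN session and opens ThirdPersonExampleMap as a listen server.
; Join connects to a given search result, and session failures only print a message.
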(event `Join`
  (params (SessionJoin :type "BlueprintSessionResult Structure"))
  (`JoinSessionCallbackProxy.JoinSession` (`GameplayStatics.GetPlayerController` 0) SessionJoin
    (:`OnFailure`
      (`KismetSystemLibrary.PrintString` "Failed"))))

(event `ShowSearchGames`
  (`/Engine/EditorBlueprintResources/StandardMacros.IsValid` (`self.SearchGames`)
    (:`Is Valid`
      _)
    (:`Is Not Valid`
      (bind _returnvalue (`|CreateWidget` "/Game/UI/SearchGame.SearchGame_C" (`GameplayStatics.GetPlayerController` 0)))
      (bind _output_get (set `self.SearchGames` _returnvalue))))
  (`UserWidget.AddToViewport` _output_get 0)
  (`UserWidget.AddToViewport` (`self.SearchGames`) 0))

(event `HostGameMenu`
  (`/Engine/EditorBlueprintResources/StandardMacros.IsValid` (`self.HostGame`)
    (:`Is Valid`
      _)
    (:`Is Not Valid`
      (bind _returnvalue (`|CreateWidget` "/Game/UI/HostGame.HostGame_C" (`GameplayStatics.GetPlayerController` 0)))
      (bind _output_get (set `self.HostGame` _returnvalue))))
  (`UserWidget.AddToViewport` _output_get 0))

(event `LaunchLobby`
  (params (`Server Name` :type Text))
  (set `self.Name` `Server Name`)
  (`CreateSessionCallbackProxy.CreateSession` (`GameplayStatics.GetPlayerController` 0) 20
    (:`OnSuccess`
      (`GameplayStatics.OpenLevel` "ThirdPersonExampleMap" true "listen"))
    (:`OnFailure`
      (`KismetSystemLibrary.PrintString` "Failed to start session"))))