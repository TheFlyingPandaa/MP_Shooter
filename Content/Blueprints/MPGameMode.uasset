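; Multiplayer game mode that tracks per-lane health, game start, player respawns and enemy spawning.
; BeginPlay gathers enemy spawn points and seeds a lane; StartGame runs once, resizing and setting lane health by player count.
; DamageLane decrements a lane's health, with debug printing.
; Authority-only events spawn and possess a new character at a fixed location, or spawn enemies at random points and edit their max health.
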(event `self.ReceiveBeginPlay`
  ;[1 1 1] Initialize Game Mode
  (`WidgetBlueprintLibrary.SetInputMode_GameOnly` (`GameplayStatics.GetPlayerController` 0))
  ;;[1 1 1] Find all and add enemy spawn points - add sort by team id
  (bind _outactors (`GameplayStatics.GetAllActorsOfClass` "/Game/Blueprints/EnemySpawnPoint.EnemySpawnPoint_C"))
  (set `self.EnemySpawnPoints` _outactors)
  ;;[1 1 1] Create Lanes - add one lane per team id
  (for _ (range 1)
    (`KismetArrayLibrary.Array_Add` (`self.LaneHealth`) 100)))

(event `DamageLane`
  (params (Lane :type Integer))
  (bind _returnvalue (- (`|GetArrayItem` (`self.LaneHealth`) Lane) 1))
  (`KismetArrayLibrary.Array_Set` (`self.LaneHealth`) Lane _returnvalue)
  ;[1 1 1] Debug print
  (`KismetSystemLibrary.PrintString` (`KismetStringLibrary.Concat_StrStr` (`KismetStringLibrary.Concat_StrStr` "Lane " (`KismetStringLibrary.Conv_IntToString` Lane)) (`KismetStringLibrary.Concat_StrStr` " have " (`KismetStringLibrary.Concat_StrStr` (`KismetStringLibrary.Conv_IntToString` _returnvalue) " HP left")))))

(event `StartGame`
  ;[0.3906 0.3906 0.3906] Game start block
  (if (`self.GameStarted?`)
    (`KismetSystemLibrary.PrintString` "Game already Started")
    (else
      (set `self.GameStarted?` true)
      (`self.setBasicInfo`))))

(event `PrintHP`
  ;[1 1 1] Print HP for every lane
  (for (_array_element _array_index) (`self.LaneHealth`)
    (`KismetSystemLibrary.PrintString` (`KismetStringLibrary.Conv_IntToString` _array_index))
    (`KismetSystemLibrary.PrintString` (`KismetStringLibrary.Conv_IntToString` _array_element))))

(event `Respawn`
  (params (Controller :type "PlayerController Object Reference"))
  ;[1 1 1] Respawn Player Pawn
  (`KismetSystemLibrary.PrintString` "gm")
  (`/Engine/EditorBlueprintResources/StandardMacros.IsValid` Controller
    (:`Is Valid`
      (`/Engine/EditorBlueprintResources/ActorMacros.Switch Has Authority`
        (:`Authority`
          (bind _returnvalue (`|SpawnActorFromClass` "/Game/Blueprints/BP_MPCharacter.BP_MPCharacter_C" (`KismetMathLibrary.MakeTransform` (-3695.0 20.0 20.0)) "AlwaysSpawn" "OverrideRootScale" null null))
          (`/Engine/EditorBlueprintResources/StandardMacros.IsValid` _returnvalue
            (:`Is Valid`
              (`Controller.Possess` Controller _returnvalue)
              (`KismetSystemLibrary.PrintString` "finished"))))))))

(event `Spawn Enemy`
  (params (`Enemy To Spawn` :type "Actor Class Reference"))
  (bind _enemyspawnpoints (`self.EnemySpawnPoints`))
  ;[1 1 1] Spawn Enemy Actor
  (`/Engine/EditorBlueprintResources/ActorMacros.Switch Has Authority`
    (:`Authority`
      (bind _returnvalue (`|SpawnActorFromClass` `Enemy To Spawn` (`self.GetTransform` (`|GetArrayItem` _enemyspawnpoints (`KismetMathLibrary.RandomInteger` (`KismetArrayLibrary.Array_Length` _enemyspawnpoints)))) "AlwaysSpawn" "OverrideRootScale" null null))
      (bind _asbp_simple_enemy (cast `/Game/Blueprints/Enemys/BP_SimpleEnemy` _returnvalue))
      (`/Game/Blueprints/Enemys/BP_SimpleEnemy.EditMaxHealth` _asbp_simple_enemy 50.0))))

(fn `setBasicInfo`
  (bind _returnvalue (`self.GetNumPlayers`))
  (bind _output_get (set `self.AmountOfPlayers` _returnvalue))
  (for _index (range _output_get)
    (`KismetArrayLibrary.Array_Set` (`self.LaneHealth`) _index 50 true)))

(fn `UserConstructionScript`
  (`parent.UserConstructionScript`))